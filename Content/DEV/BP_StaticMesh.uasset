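; A configurable static mesh actor that lets each placed instance pick its mesh, material and look from exposed-style variables.
; The construction script applies the mesh and slot 0 material, then pushes top and side color pairs, tiling and roughness into the material parameters.
; It has no runtime logic, as its event graph holds only disabled default events.
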(event EventBeginPlay)

(event Collision|EventActorBeginOverlap
  (params (OtherActor :type Actor%20Object%20Reference)))

(event EventTick
  (params (DeltaSeconds :type Float%20%28single-precision%29)))

(fn ConstructionScript
  (Components|StaticMesh|SetStaticMesh (Variables|Default|GetStaticMesh) (Variables|MeshParameters|GetMesh))
  (Rendering|Material|SetMaterial (Variables|Default|GetStaticMesh) 0 (Variables|MeshParameters|GetMaterial))
  (Rendering|Material|SetVectorParameterValueonMaterials (Variables|Default|GetStaticMesh) "TopColor_1" (Math|Conversions|ToVector(LinearColor) (Variables|MeshParameters|GetTop_Color_1)))
  (Rendering|Material|SetVectorParameterValueonMaterials (Variables|Default|GetStaticMesh) "TopColor_2" (Math|Conversions|ToVector(LinearColor) (Variables|MeshParameters|GetTop_Color_2)))
  (Rendering|Material|SetVectorParameterValueonMaterials (Variables|Default|GetStaticMesh) "SideColor_1" (Math|Conversions|ToVector(LinearColor) (Variables|MeshParameters|GetSide_Color_1)))
  (Rendering|Material|SetVectorParameterValueonMaterials (Variables|Default|GetStaticMesh) "SideColor_2" (Math|Conversions|ToVector(LinearColor) (Variables|MeshParameters|GetSide_Color_2)))
  (Rendering|Material|SetScalarParameterValueonMaterials (Variables|Default|GetStaticMesh) "Tiling" (Variables|MeshParameters|GetTiling))
  (Rendering|Material|SetScalarParameterValueonMaterials (Variables|Default|GetStaticMesh) "Roughness" (Variables|MeshParameters|GetRoughness)))